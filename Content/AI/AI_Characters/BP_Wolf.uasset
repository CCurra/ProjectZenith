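; BP_Wolf is an AI wolf with a melee hitbox that kills any other BP_Wolf it overlaps.
; DoAttack switches the hitbox's query collision on or off, and the overlap event calls OnDeath on the wolf it hits.
; OnDeath runs once, disabling the hitbox, stopping the AI controller's brain logic and destroying the actor after a short delay.
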(event `self.hitbox.OnComponentBeginOverlap`
  (params (OverlappedComponent :type "PrimitiveComponent Object Reference") (OtherActor :type "Actor Object Reference") (OtherComp :type "PrimitiveComponent Object Reference") (OtherBodyIndex :type Integer) (bFromSweep :type Boolean) (SweepResult :type "HitResult Structure (by ref)"))
  (bind _asbp_wolf (cast `/Game/AI/AI_Characters/BP_Wolf` OtherActor))
  (`self.OnDeath` _asbp_wolf))

(event `OnDeath`
  (if (not (`self.isDead`))
    (`PrimitiveComponent.SetCollisionEnabled` (`self.hitbox`) "NoCollision")
    (set `self.isDead` true)
    (`BrainComponent.StopLogic` (`AIController.BrainComponent` (`AIBlueprintHelperLibrary.GetAIController` self)) "")
    (`KismetSystemLibrary.Delay` 1.5)
    (`self.K2_DestroyActor`)))

(fn `Do Attack`
  (params (isAttacking :type Boolean))
  (bind _hitbox (`self.hitbox`))
  (if isAttacking
    (`PrimitiveComponent.SetCollisionEnabled` _hitbox "QueryOnly")
    (else
      (`PrimitiveComponent.SetCollisionEnabled` _hitbox "NoCollision")
      (set `self.isAttacking` false))))

(fn `UserConstructionScript`)