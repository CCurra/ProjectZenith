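; Player character Blueprint for the Doll, with side-scroller style movement, crouching and a HUD.
; The MoveRight axis drives movement along a fixed world Y axis, with positive input heading toward negative Y.
; The Crouch action works as a toggle through a Crouching boolean, and BeginPlay creates the Doll_Hud widget for the first player controller and adds it to the viewport.
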(event `InputAxis|MoveRight`
  (params (AxisValue :type "Float (single-precision)"))
  ;[1 1 1] Movement
  (`self.AddMovementInput` (0.0 -1.0 0.0) AxisValue))

(event `InputAction|Crouch`
  (params (Key :type "Key Structure"))
  ;[1 1 1] Crouch
  (:`Pressed`
    (if (`self.Crouching`)
      (set `self.Crouching` false)
      (`self.UnCrouch`)
      (else
        (set `self.Crouching` true)
        (`self.Crouch`)))))

(event `self.ReceiveBeginPlay`
  ;[1 1 1] Hud
  (bind _returnvalue (`|CreateWidget` "/Game/Widgets/HUD/Doll_Hud.Doll_Hud_C" (`GameplayStatics.GetPlayerController` 0)))
  (`UserWidget.AddToViewport` _returnvalue 0))

(fn `UserConstructionScript`)