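; Playable Jack-in-the-box character with a mouse-aimed grapple, able to swap into ActionFigure or BP_Horse pawns on number keys.
; Holding left mouse traces under the cursor for a nearby hook point, then Tick extends a child-actor cable toward it.
; A single LaunchCharacter per press fakes the swing, using cursor offset from a hard-coded screen centre; release resets it.
; G destroys the first Grabbable found at BeginPlay, if interactable.
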(event `self.ReceivePossessed`
  (params (NewController :type "Controller Object Reference"))
  (set `PlayerController.bShowMouseCursor` true (`GameplayStatics.GetPlayerController` 0)))

(event `self.ReceiveBeginPlay`
  ;[1 1 1] Comment
  (set `PlayerController.bEnableMouseOverEvents` true (`GameplayStatics.GetPlayerController` 0))
  (bind _ascable_actor (cast `CableActor` (`ChildActorComponent.ChildActor` (`self.CableActor`))))
  (bind _cablecomponent (`CableActor.CableComponent` _ascable_actor))
  (`SceneComponent.SetVisibility` _cablecomponent false false)
  (set `CableComponent.CableWidth` 10.0 _cablecomponent)
  (set `CableComponent.EndLocation` (0.0 0.0 0.0) _cablecomponent)
  (set `CableComponent.CableLength` 0.0 _cablecomponent)
  (set `CableComponent.SolverIterations` 2 _cablecomponent)
  (set `self.grappleCmpnt` _cablecomponent)
  (bind _outactors (`GameplayStatics.GetAllActorsOfClass` "/Game/Blueprints/JackInTheBox/Grabbable.Grabbable_C"))
  (set `self.Grabbable` (`|GetArrayItem` _outactors))
  (bind _outactors_2 (`GameplayStatics.GetAllActorsOfClass` "/Game/Blueprints/JackInTheBox/Grapple.Grapple_C"))
  (set `self.Grapple` (`|GetArrayItem` _outactors_2))
  (bind _outactors_3 (`GameplayStatics.GetAllActorsOfClass` "/Game/Blueprints/JackInTheBox/GrappleDestination.GrappleDestination_C"))
  (set `self.GrapplePoint` (`|GetArrayItem` _outactors_3)))

(event `self.ReceiveTick`
  (params (DeltaSeconds :type "Float (single-precision)"))
  (bind _returnvalue (`GameplayStatics.GetPlayerController` 0))
  (bind _grappledistance (`self.grappleDistance`))
  (bind _lasthook (`self.lastHook`))
  (bind _grapplecmpnt (`self.grappleCmpnt`))
  (bind (_hitresult _returnvalue_2) (`PlayerController.GetHitResultUnderCursorByChannel` _returnvalue "TraceTypeQuery1" false))
  (bind (_locationx _locationy) (`PlayerController.GetMousePosition` (`GameplayStatics.GetPlayerController` 0)))
  (bind _endlocation (`CableComponent.EndLocation` _grapplecmpnt))
  (bind _returnvalue_3 (`KismetMathLibrary.LessLess_VectorRotator` (- _lasthook (`self.K2_GetActorLocation`)) (`self.K2_GetActorRotation`)))
  (bind _returnvalue_4 (- _locationy 359.5))
  (bind (_bblockinghit _binitialoverlap _time _distance _location) (`GameplayStatics.BreakHitResult` _hitresult))
  ;[1 1 1] Grapple Hook
  (set `self.Delta Time` DeltaSeconds)
  (`|ExecutionSequence`
    (:`then_0`
      (if (and (`PlayerController.IsInputKeyDown` _returnvalue "LeftMouseButton") (== (`self.lastHook`) (0.0 0.0 0.0)) (`self.canGrapple`))
        (if (and _returnvalue_2 (< (`KismetMathLibrary.VSize` (- (`self.K2_GetActorLocation`) _location)) 1000.0))
          ;[1 1 1] Update Hook
          (set `self.lastHook` _location))))
    (:`then_1`
      ;[1 1 1] Updating End Hook Location
      (if (and (`PlayerController.IsInputKeyDown` _returnvalue "LeftMouseButton") (!= _lasthook (0.0 0.0 0.0)))
        (if (`self.hooked`)
          (set `self.HookLocation` _returnvalue_3)
          (set `CableComponent.EndLocation` _returnvalue_3 _grapplecmpnt)
          (else
            (set `CableComponent.EndLocation` (`KismetMathLibrary.VInterpTo` _endlocation _returnvalue_3 (`self.Delta Time`) 1.0) _grapplecmpnt)))
        (if (> (`KismetMathLibrary.VSize` (- _returnvalue_3 _endlocation)) (* _grappledistance 0.99))
          (set `self.hooked` true)
          (elif false
            (set `self.grappleDistance` 10.0)
            (elif (< _grappledistance 1500.0)
              (set `CableComponent.SolverIterations` 1 (`self.grappleCmpnt`)))))))
    (:`then_2`
      ;[1 1 1] Move Character to hook
      (if (and (`PlayerController.IsInputKeyDown` (`GameplayStatics.GetPlayerController` 0) "LeftMouseButton") (!= (`self.lastHook`) (0.0 0.0 0.0)))
        (`KismetSystemLibrary.PrintString` (`KismetStringLibrary.Conv_DoubleToString` (`CableComponent.CableLength` (`self.Cable`))))
        (`|ExecutionSequence`
          (:`then_0`
            (if (not (`self.IS Swinging`))
              (`|ExecutionSequence`
                (:`then_0`
                  (if (>= 0.0 (- _locationx 639.5))
                    (bind _result (`/Engine/EditorBlueprintResources/StandardMacros.NegateFloat` _returnvalue_4)
                      (:`  `
                        (`SceneComponent.SetVisibility` (`self.grappleCmpnt`) true false)
                        (`self.LaunchCharacter` (`KismetMathLibrary.MakeVector` 0.0 1300.0 (* _result 2.0)) true true)
                        (set `self.IS Swinging` true)))
                    (else
                      (bind _result_2 (`/Engine/EditorBlueprintResources/StandardMacros.NegateFloat` _returnvalue_4)
                        (:`  `
                          (`SceneComponent.SetVisibility` (`self.grappleCmpnt`) true false)
                          (`self.LaunchCharacter` (`KismetMathLibrary.MakeVector` 0.0 -1300.0 (* _result_2 2.0)) true true)
                          (set `self.IS Swinging` true))))))))))))))

(event `Key|LeftMouseButton`
  (params (Key :type "Key Structure"))
  (bind _grapplecmpnt (`self.grappleCmpnt`))
  (:`Released`
    ;[1 1 1] Reset Hook
    (set `self.lastHook` (0.0 0.0 0.0))
    (set `CableComponent.EndLocation` (0.0 0.0 0.0) _grapplecmpnt)
    (set `CableComponent.SolverIterations` 5 _grapplecmpnt)
    (`SceneComponent.SetVisibility` _grapplecmpnt false false)
    (set `self.IS Swinging` false)))

(event `Key|One`
  (params (Key :type "Key Structure"))
  (:`Pressed`
    (`self.Switch to Action Figure`)))

(event `Key|Two`
  (params (Key :type "Key Structure"))
  (:`Pressed`
    (`self.Switch to Horse`)))

(event `Key|G`
  (params (Key :type "Key Structure"))
  ;[1 1 1] Grabbable objects
  (:`Pressed`
    (bind _asgrabbable (cast `/Game/Blueprints/JackInTheBox/Grabbable` (`self.Grabbable`)))
    (if (`/Game/Blueprints/JackInTheBox/Grabbable.IsInteractable` _asgrabbable)
      (`self.K2_DestroyActor` _asgrabbable))))

(event `Key|Three`
  (params (Key :type "Key Structure"))
  ;[1 1 1] Not sure its needed can reconnect if needed
)

(event `Key|I`
  (params (Key :type "Key Structure")))

(fn `Stay as Jack`)

(fn `Switch to Action Figure`
  (bind _returnvalue (`GameplayStatics.GetPlayerController` 0))
  (`Controller.UnPossess` _returnvalue)
  (`self.K2_DestroyActor`)
  (bind _returnvalue_2 (`|SpawnActorFromClass` "/Game/Blueprints/ActionFigure.ActionFigure_C" (`self.GetTransform` _returnvalue) "AlwaysSpawn" "OverrideRootScale" null null))
  (`self.K2_TeleportTo` _returnvalue_2 (`self.K2_GetActorLocation`) (`self.K2_GetActorRotation`))
  (`Controller.Possess` (`GameplayStatics.GetPlayerController` 0) _returnvalue_2))

(fn `Switch to Horse`
  (bind _returnvalue (`GameplayStatics.GetPlayerController` 0))
  (`Controller.UnPossess` _returnvalue)
  (`self.K2_DestroyActor`)
  (bind _returnvalue_2 (`|SpawnActorFromClass` "/Game/Blueprints/BP_Horse.BP_Horse_C" (`self.GetTransform` _returnvalue) "AlwaysSpawn" "OverrideRootScale" null null))
  (`self.K2_TeleportTo` _returnvalue_2 (`self.K2_GetActorLocation`) (`self.K2_GetActorRotation`))
  (`Controller.Possess` (`GameplayStatics.GetPlayerController` 0) _returnvalue_2))

(fn `UserConstructionScript`)