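; Pressure plate Blueprint that sinks when something overlaps its Box and opens a linked Door_Blueprint.
; A timeline lerps the ChildActor between UpPosition and DownPosition, playing on begin overlap and reversing on end overlap.
; End overlap calls PlateUp again after a short delay, and nothing here closes the door.
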(event `Plate Down`
  (bind (_direction _driver) (`Timeline|Timeline_0` :!label _label)
    (:`Update`
      (`SceneComponent.K2_SetRelativeLocation` (`self.ChildActor`) (`KismetMathLibrary.VLerp` (`self.UpPosition`) (`self.DownPosition`) _driver) false false))))

(event `Plate Up`
  (goto _label :!via `Reverse`))

(event `self.Box.OnComponentBeginOverlap`
  (params (OverlappedComponent :type "PrimitiveComponent Object Reference") (OtherActor :type "Actor Object Reference") (OtherComp :type "PrimitiveComponent Object Reference") (OtherBodyIndex :type Integer) (bFromSweep :type Boolean) (SweepResult :type "HitResult Structure (by ref)"))
  (`self.Plate Down`)
  (bind _asdoor_blueprint (cast `/Game/Blueprints/doors/Door_Blueprint` (`self.Door Component`)))
  (`/Game/Blueprints/doors/Door_Blueprint.DoorOpen` _asdoor_blueprint))

(event `self.Box.OnComponentEndOverlap`
  (params (OverlappedComponent :type "PrimitiveComponent Object Reference") (OtherActor :type "Actor Object Reference") (OtherComp :type "PrimitiveComponent Object Reference") (OtherBodyIndex :type Integer))
  (`self.Plate Up`)
  (`KismetSystemLibrary.Delay` 1.0)
  (`self.Plate Up`))

(fn `UserConstructionScript`)