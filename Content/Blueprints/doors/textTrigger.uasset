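; An interactable trigger Blueprint that shows or hides a text label and opens a linked door or trap door.
; Entering or leaving TextCollider toggles the TextRender's visibility.
; Interact alternates through a FlipFlop: one press sets Active and calls DoorOpen on SecondComponent, cast as TrapDoor_Blueprint or Door_Blueprint.
; The next press only clears Active without closing anything, and both presses print the state.
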(event `self.textCollider.OnComponentBeginOverlap`
  (params (OverlappedComponent :type "PrimitiveComponent Object Reference") (OtherActor :type "Actor Object Reference") (OtherComp :type "PrimitiveComponent Object Reference") (OtherBodyIndex :type Integer) (bFromSweep :type Boolean) (SweepResult :type "HitResult Structure (by ref)"))
  (`SceneComponent.ToggleVisibility` (`self.TextRender`) false))

(event `/Game/Blueprints/InteractionInterface.Interact`
  (params (Player :type "Actor Object Reference"))
  (`/Engine/EditorBlueprintResources/StandardMacros.FlipFlop`
    (:`A`
      (bind _output_get (set `self.Active` true))
      (`KismetSystemLibrary.PrintString` (`KismetStringLibrary.Conv_BoolToString` _output_get))
      (bind _astrap_door_blueprint (cast `/Game/Blueprints/doors/TrapDoor_Blueprint` (`self.second component`))
        (:`then`
          (`/Game/Blueprints/doors/TrapDoor_Blueprint.DoorOpen` _astrap_door_blueprint))
        (:`CastFailed`
          _))
      (bind _asdoor_blueprint (cast `/Game/Blueprints/doors/Door_Blueprint` (`self.second component`)))
      (`/Game/Blueprints/doors/Door_Blueprint.DoorOpen` _asdoor_blueprint))
    (:`B`
      (bind _output_get_2 (set `self.Active` false))
      (`KismetSystemLibrary.PrintString` (`KismetStringLibrary.Conv_BoolToString` _output_get_2)))))

(event `self.textCollider.OnComponentEndOverlap`
  (params (OverlappedComponent :type "PrimitiveComponent Object Reference") (OtherActor :type "Actor Object Reference") (OtherComp :type "PrimitiveComponent Object Reference") (OtherBodyIndex :type Integer))
  (`SceneComponent.ToggleVisibility` (`self.TextRender`) false))

(fn `UserConstructionScript`)