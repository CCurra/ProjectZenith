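; Projectile actor for the ActionFigure asset that damages whatever it overlaps, other than its owner, then destroys itself.
; Overlap on the Projectile component applies BaseDamage of the configured DamageType with itself as damage causer.
; It credits the owner's instigator controller when valid, relying on the owner set at spawn, and otherwise applies damage without an instigator.
; On BeginPlay it also schedules self-destruction after DestroyTime.
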(event `self.Projectile.OnComponentBeginOverlap`
  (params (OverlappedComponent :type "PrimitiveComponent Object Reference") (OtherActor :type "Actor Object Reference") (OtherComp :type "PrimitiveComponent Object Reference") (OtherBodyIndex :type Integer) (bFromSweep :type Boolean) (SweepResult :type "HitResult Structure (by ref)"))
  (bind _basedamage (`self.BaseDamage`))
  (bind _damagetype (`self.DamageType`))
  (bind _returnvalue (`self.GetInstigatorController` (`self.GetOwner`)))
  (if (!= (`self.GetOwner`) OtherActor)
    (`/Engine/EditorBlueprintResources/StandardMacros.IsValid` _returnvalue
      (:`Is Valid`
        (`GameplayStatics.ApplyDamage` OtherActor _basedamage _returnvalue self _damagetype) ; Instigator is valid
        (`self.K2_DestroyActor`))
      (:`Is Not Valid`
        (`GameplayStatics.ApplyDamage` OtherActor _basedamage null self _damagetype) ; Fall Back, do not get instigator
        (`self.K2_DestroyActor`)))))

(event `self.ReceiveBeginPlay`
  (`KismetSystemLibrary.Delay` (`self.DestroyTime`))
  (`self.K2_DestroyActor`))

(fn `UserConstructionScript`)